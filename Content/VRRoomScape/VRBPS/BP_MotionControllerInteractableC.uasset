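; VR motion controller hand actor that grabs and releases nearby interactable actors and animates its hand mesh.
; Trigger press finds the nearest interactable and sends it a pickup message with the motion controller; release sends a drop message.
; Grip, trigger, free-hand and controller state are pushed to the hand's Animation Blueprint, cached on BeginPlay.
; The construction script calls InvertHandMotion unless the hand starts as left.
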(event EventBeginPlay
  (bind _ashand_lp_skeleton_anim_blueprint (Utilities|Casting|CastToHandLP_Skeleton_AnimBlueprint (Components|SkeletalMesh|GetAnimInstance (Variables|Default|GethandMesh))))
  (Variables|Default|SetHandLPAnimBP _ashand_lp_skeleton_anim_blueprint))

(fn ConstructionScript
  (if (not (Variables|Default|GetstartAsLeftHand))
    (Class|MotionControllerInteractable|InvertHandMotion)))

(fn SetGrip
  (params (bIsGripPressed :type Boolean))
  (Variables|Default|SetbIsGripPressed bIsGripPressed)
  (Animation|UpdateAnimation))

(fn SetTrigger
  (params (TriggerPress :type Boolean))
  (bind _output_get (Variables|Default|SetbIsTriggerPressed TriggerPress))
  (if _output_get
    (if (not (Variables|Default|GetbIsGrabbing))
      (bind _returnvalue (Class|MotionControllerInteractable|GetNearInteractable))
      (Variables|Default|SetNearestPickupActor _returnvalue)
      (bind _nearestpickupactor (Variables|Default|GetNearestPickupActor)
        (:then
          (Interactors|GrabActor _nearestpickupactor)
          (Variables|Default|SetbIsGrabbing true)
          (Variables|Default|SetcontrollerState "Grab"))
        (:else
          _))
      (Animation|UpdateAnimation :!label _label))
    (elif (Variables|Default|GetbIsGrabbing)
      (Interactors|ReleaseActor)
      (Variables|Default|SetbIsGrabbing false)
      (Variables|Default|SetcontrollerState "Open")
      (goto _label)
      (else
        (goto _label)))))

(fn GrabActor
  (params (Actor :type Actor%20Object%20Reference))
  (Utilities|IsValid Actor
    (:Is%20Valid
      (bind _output_get (Variables|Default|SetAttachedActor Actor))
      (Class|PickupInterface|Pickup(Message) _output_get (Variables|Default|GetmotionController))
      (Variables|Default|SetcontrollerState "Grab"))))

(fn ReleaseActor
  (Variables|Default|SetcontrollerState "Open")
  (bind _attachedactor (Variables|Default|GetAttachedActor)
    (:then
      (Class|PickupInterface|Drop(Message) _attachedactor (Variables|Default|GetmotionController))
      (Variables|Default|SetAttachedActor 0))
    (:else
      _))
  (Variables|Default|SetbIsGrabbing false))

(fn UpdateAnimation
  (bind _handlpanimbp (Variables|Default|GetHandLPAnimBP))
  (Utilities|FlowControl|Sequence
    (:then_0
      (Variables|/Game/VRRoomScape/Hand/HandLP_Skeleton_AnimBlueprint.HandLP_Skeleton_AnimBlueprint_C|SetbIsFreeHand _handlpanimbp (not (Variables|Default|GetbIsGrabbing))))
    (:then_1
      (Variables|/Game/VRRoomScape/Hand/HandLP_Skeleton_AnimBlueprint.HandLP_Skeleton_AnimBlueprint_C|SetbIsGripPressed _handlpanimbp (Variables|Default|GetbIsGripPressed)))
    (:then_2
      (Variables|/Game/VRRoomScape/Hand/HandLP_Skeleton_AnimBlueprint.HandLP_Skeleton_AnimBlueprint_C|SetbIsTriggerPressed _handlpanimbp (Variables|Default|GetbIsTriggerPressed)))
    (:then_3
      (Variables|/Game/VRRoomScape/Hand/HandLP_Skeleton_AnimBlueprint.HandLP_Skeleton_AnimBlueprint_C|SetController%20State _handlpanimbp (Variables|Default|GetcontrollerState)))))