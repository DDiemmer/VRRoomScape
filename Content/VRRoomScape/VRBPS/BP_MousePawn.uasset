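; Free-moving pawn that switches between mouse look and a cursor-driven grab mode with the G key, for dragging objects in the world.
; In grab mode, a left-click traces from the cursor and picks up Movable components, storing hit distance and local grab offset.
; Each tick, physics bodies, including skeletal mesh bones, follow the cursor at that distance through a PhysicsHandle with a debug line, while non-simulating components are repositioned directly.
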(event EventTick
  (params (DeltaSeconds :type Float%20%28single-precision%29))
  (bind _returnvalue (Game|GetPlayerController 0))
  (bind _grabbedcomponent (Variables|Default|GetgrabbedComponent))
  (bind _originaldistancetoobject (Variables|Default|GetoriginalDistanceToObject))
  (bind (_worldlocation _worlddirection) (Game|Player|ConvertMouseLocationToWorldSpace _returnvalue))
  (bind _returnvalue_2 (* _worlddirection _originaldistancetoobject))
  (bind _returnvalue_3 (+ _worldlocation _returnvalue_2))
  ;[1 1 1] Event tick
  (if (Variables|Default|Getb_grabMode)
    (Utilities|IsValid (Variables|Default|GetgrabbedComponent)
      (:Is%20Valid
        (if (Physics|IsSimulatingPhysics (Variables|Default|GetgrabbedComponent) "None")
          (Physics|Components|PhysicsHandle|SetTargetLocation (Variables|Default|GetPhysicsHandle) _returnvalue_3)
          (Rendering|Debug|DrawDebugLine _returnvalue_3 (Math|Transform|TransformLocation (select (Variables|Default|Getb_skeletalMesh) (Transformation|GetSocketTransform _grabbedcomponent (Variables|Default|GetboneName) "RTS_World") (Transformation|GetWorldTransform _grabbedcomponent)) (Variables|Default|GetrelativeGrabLocation)) "(R=0.668435,G=0.000000,B=1.000000,A=1.000000)" 0.0 5.0)
          (else
            (Transformation|SetWorldLocation (Variables|Default|GetgrabbedComponent) (Math|Transform|InverseTransformLocation (Math|Conversions|ToTransform(Vector) (Variables|Default|GetrelativeGrabLocation)) _returnvalue_3) false false)))))))

(event Input|AxisEvents|InputAxisTurn
  (params (AxisValue :type Float%20%28single-precision%29))
  ;[1 1 1] Update pawn Location
  (if (not (Variables|Default|Getb_grabMode))
    (Pawn|Input|AddControllerYawInput AxisValue)))

(event Input|AxisEvents|InputAxisLookUp
  (params (AxisValue :type Float%20%28single-precision%29))
  ;[1 1 1] Update pawn Location
  (if (not (Variables|Default|Getb_grabMode))
    (Pawn|Input|AddControllerPitchInput (* -1 AxisValue))))

(event Input|AxisEvents|InputAxisMoveRight
  (params (AxisValue :type Float%20%28single-precision%29))
  ;[1 1 1] Move Pawn
  (if (!= AxisValue 0.0)
    (Transformation|AddActorWorldOffset (* (Math|Vector|GetRightVector (Transformation|GetActorRotation (Pawn|GetController))) (* AxisValue -1e+01)))))

(event Input|AxisEvents|InputAxisMovForward
  (params (AxisValue :type Float%20%28single-precision%29))
  ;[1 1 1] Move Pawn
  (if (!= AxisValue 0.0)
    (Transformation|AddActorWorldOffset (* (Math|Vector|GetForwardVector (Transformation|GetActorRotation (Pawn|GetController))) (* AxisValue 1e+01)))))

(event Input|KeyboardEvents|G
  (params (Key :type Key%20Structure :default "None"))
  (bind _returnvalue (Game|GetPlayerController 0))
  ;[1 1 1] Activate Mouse Pointer
  (:Pressed
    (Variables|Default|Setb_grabMode (not (Variables|Default|Getb_grabMode)))
    (bind _output_get (Variables|/Script/Engine.PlayerController|SetbShowMouseCursor _returnvalue (not (Variables|/Script/Engine.PlayerController|GetbShowMouseCursor _returnvalue))))
    (Development|PrintString (Utilities|String|Append "Mouse Grab:" (Utilities|String|ToString(Boolean) _output_get)))))

(event Input|MouseEvents|LeftMouseButton
  (params (Key :type Key%20Structure :default "None"))
  (bind _returnvalue (Game|GetPlayerController 0))
  (bind _b_grabmode (Variables|Default|Getb_grabMode))
  (bind (_worldlocation _worlddirection) (Game|Player|ConvertMouseLocationToWorldSpace _returnvalue))
  ;[1 1 1] Mouse Collision with object
  (:Pressed
    (if _b_grabmode
      (bind (_outhit _returnvalue_2) (Collision|LineTraceByChannel _worldlocation (+ _worldlocation (* _worlddirection (Math|Float|MakeLiteralFloat 1e+04))) "TraceTypeQuery1" true 0 "ForDuration"))
      (if _returnvalue_2
        (if (== (Variables|/Script/Engine.SceneComponent|GetMobility (.HitComponent (Collision|BreakHitResult _outhit))) (Utilities|Enum|LiteralenumEComponentMobility "Movable"))
          (Variables|Default|SetoriginalDistanceToObject (.Distance (Collision|BreakHitResult _outhit)))
          (bind _output_get (Variables|Default|SetgrabbedComponent (.HitComponent (Collision|BreakHitResult _outhit))))
          (if (Physics|IsSimulatingPhysics _output_get "None")
            (Utilities|Casting|CastToSkeletalMeshComponent (Variables|Default|GetgrabbedComponent)
              (:then
                (Variables|Default|Setb_skeletalMesh true)
                (Variables|Default|SetboneName (.HitBoneName (Collision|BreakHitResult _outhit))))
              (:CastFailed
                _))
            (Class|PhysicsHandleComponent|GrabComponentatLocation (Variables|Default|GetPhysicsHandle) (Variables|Default|GetgrabbedComponent) (Variables|Default|GetboneName) (.Location (Collision|BreakHitResult _outhit)))
            (Variables|Default|SetrelativeGrabLocation (Math|Transform|InverseTransformLocation (select (Variables|Default|Getb_skeletalMesh) (Transformation|GetSocketTransform (Variables|Default|GetgrabbedComponent) (Variables|Default|GetboneName) "RTS_World") (Transformation|GetWorldTransform (Variables|Default|GetgrabbedComponent))) (.Location (Collision|BreakHitResult _outhit))))
            (else
              (Variables|Default|SetrelativeGrabLocation (Math|Transform|InverseTransformLocation (Math|Conversions|ToTransform(Vector) (Transformation|GetWorldLocation (.HitComponent (Collision|BreakHitResult _outhit)))) (.Location (Collision|BreakHitResult _outhit))))))))))
  (:Released
    (if _b_grabmode
      (Variables|Default|SetgrabbedComponent 0)
      (Physics|Components|PhysicsHandle|ReleaseComponent (Variables|Default|GetPhysicsHandle)))))

(fn ConstructionScript)