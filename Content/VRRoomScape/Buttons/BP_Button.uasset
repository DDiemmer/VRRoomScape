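; BP_Button is a glowing, colored button actor that plays a click sound when its Button component stops overlapping BoxClick.
; The construction script creates a dynamic glow material tinted with ButtonColor.
; GlowButton raises the material's Bloom and, given a positive time, calls DarkButtonEvent to dim it after a delay.
; A test loop in that event then glows again with a random duration, so flashing repeats indefinitely once started.
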(event OnComponentEndOverlap(BoxClick)
  (params (OverlappedComponent :type Primitive%20Component%20Object%20Reference) (OtherActor :type Actor%20Object%20Reference) (OtherComp :type Primitive%20Component%20Object%20Reference) (OtherBodyIndex :type Integer))
  (bind _button (Variables|Default|GetButton))
  (if (== OtherComp _button)
    (Audio|PlaySoundatLocation "/Game/VRRoomScape/Audio/buttonclick.buttonclick" (Transformation|GetWorldLocation _button) "0, 0, 0" 1.0 1.0 0.0 0 0 0)))

(event Custom|DarkButtonEvent
  (params (timeToDark :type Float%20%28single-precision%29) (minBloomValue :type Float%20%28single-precision%29))
  (Utilities|FlowControl|Delay timeToDark)
  (CallFunction|DarkButton minBloomValue)
  ;[1 1 1] test loop
  (Utilities|FlowControl|Delay timeToDark)
  (CallFunction|GlowButton 7.0 (Math|Random|RandomFloatinRange 0.12 5.0) 0.0))

(event EventBeginPlay)

(event Collision|EventActorBeginOverlap
  (params (OtherActor :type Actor%20Object%20Reference)))

(event EventTick
  (params (DeltaSeconds :type Float%20%28single-precision%29)))

(fn ConstructionScript
  (bind _returnvalue (Rendering|Material|CreateDynamicMaterialInstance (Variables|Default|GetButton) 0 "/Game/VRRoomScape/Materials/MI_GlowBase.MI_GlowBase" "None" :!class /Script/Engine.PrimitiveComponent))
  (Rendering|Material|SetVectorParameterValue _returnvalue "BaseColor" (Variables|ButtonAttributes|GetButtonColor) :!class /Script/Engine.MaterialInstanceDynamic)
  (Variables|ButtonAttributes|SetbuttonMaterial _returnvalue))

(fn GlowButton
  (params (MaxBloomValue :type Float%20%28single-precision%29) (TimeToDarke :type Float%20%28single-precision%29) (minBloomValue :type Float%20%28single-precision%29))
  (Rendering|Material|SetScalarParameterValue (Variables|ButtonAttributes|GetbuttonMaterial) "Bloom" MaxBloomValue :!class /Script/Engine.MaterialInstanceDynamic)
  (if (> TimeToDarke 0.0)
    (CallFunction|DarkButtonEvent TimeToDarke minBloomValue)))

(fn DarkButton
  (params (MinBloomValue :type Float%20%28single-precision%29))
  (Rendering|Material|SetScalarParameterValue (Variables|ButtonAttributes|GetbuttonMaterial) "Bloom" MinBloomValue :!class /Script/Engine.MaterialInstanceDynamic))